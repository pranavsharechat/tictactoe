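; Player controller for a tic-tac-toe game that sets up the player's UI and relays turn events, with separate online and offline modes.
; On BeginPlay it creates the online widget for networked non-dedicated instances and submits the name from the game instance, or creates the offline widget in standalone.
; AuthenticatePlayer updates the online widget's text and toggles the mouse cursor.
; PlayerTurnPlayed notifies the game mode that the turn is over.
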(event Custom|AuthenticatePlayer
  (params (bAllowed :type Boolean))
  (bind _onlineuiwidget (Variables|Default|GetOnlineUIWidget))
  (Utilities|IsValid _onlineuiwidget
    (:Is%20Valid
      (Default|UpdateGameText _onlineuiwidget bAllowed)
      (if bAllowed
        (Variables|Default|SetbShowMouseCursor true)
        (else
          (Variables|Default|SetbShowMouseCursor false))))))

(event Custom|PlayerTurnPlayed
  (bind _astic_tac_toe_game_mode_bp (Utilities|Casting|CastToTicTacToeGameModeBP (Game|GetGameMode)))
  (Default|PlayerTurnOveronGameMode _astic_tac_toe_game_mode_bp))

(event EventBeginPlay
  (Utilities|FlowControl|Sequence
    (:then_0
      (if (and (not (Networking|IsDedicatedServer)) (not (Class|KismetSystemLibrary|IsStandalone)))
        (Utilities|FlowControl|Sequence
          (:then_0
            (bind _returnvalue (UserInterface|CreateWidget "/Game/PlayerUI.PlayerUI_C" (Game|GetPlayerController 0)))
            (UserInterface|Viewport|AddtoViewport _returnvalue 0)
            (Variables|Default|SetOnlineUIWidget _returnvalue))
          (:then_1
            (bind _astic_tac_toe_game_instance (Utilities|Casting|CastToTicTacToeGameInstance (Game|GetGameInstance)))
            (Class|TTTPlayerController|SetPlayerInfo (Variables|/Script/TicTacToe.TicTacToeGameInstance|GetPlayerName _astic_tac_toe_game_instance))))))
    (:then_1
      (if (Class|KismetSystemLibrary|IsStandalone)
        (bind _returnvalue_2 (UserInterface|CreateWidget "/Game/OflineUI.OflineUI_C" (Game|GetPlayerController 0)))
        (UserInterface|Viewport|AddtoViewport _returnvalue_2 0)))))

(event EventTick
  (params (DeltaSeconds :type Float%20%28single-precision%29)))

(fn ConstructionScript)