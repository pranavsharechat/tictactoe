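; Game mode for a two-player networked Tic-Tac-Toe match that decides whose turn it is.
; PostLogin registers each player controller with input unauthenticated and starts the game on a short timer at two players; logout removes the controller.
; A FlipFlop alternates which controller is authenticated to play; when a turn ends, both are revoked and the next follows after a delay.
; A looping timer prints the player count for debugging.
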(event Custom|CustomEvent
  (Development|PrintString (Utilities|String|Append "No of Players: " (Utilities|String|ToString(Integer) (Utilities|Array|Length (Variables|/Script/Engine.GameStateBase|GetPlayerArray (Game|GetGameState)))))))

(event Custom|StartGame
  (Development|PrintString "Choosing Players...")
  (CallFunction|StartPlayerTurn))

(event Custom|Start%20Player%20Turn
  (Utilities|FlowControl|FlipFlop
    (:A
      (Default|AuthenticatePlayer (Utilities|Array|Get(acopy) (Variables|Default|GetPlayerControllerList)) true)
      (Default|AuthenticatePlayer (Utilities|Array|Get(acopy) (Variables|Default|GetPlayerControllerList) 1) false))
    (:B
      (Default|AuthenticatePlayer (Utilities|Array|Get(acopy) (Variables|Default|GetPlayerControllerList)) false)
      (Default|AuthenticatePlayer (Utilities|Array|Get(acopy) (Variables|Default|GetPlayerControllerList) 1) true))))

(event Custom|PlayerTurnOver_OnGameMode
  (Development|PrintString "Player Turn Played. Will Pick Another Player for Turn in Sometime")
  (Default|AuthenticatePlayer (Utilities|Array|Get(acopy) (Variables|Default|GetPlayerControllerList)) false)
  (Utilities|Time|SetTimerbyEvent (delegate Custom|Start%20Player%20Turn) 2.0))

(event EventBeginPlay
  (Utilities|Time|SetTimerbyEvent (delegate Custom|CustomEvent) 2.0 true))

(event EventTick
  (params (DeltaSeconds :type Float%20%28single-precision%29)))

(event EventPostLogin
  (params (NewPlayer :type Player%20Controller%20Object%20Reference))
  (bind _astttplayer_controller_bp (Utilities|Casting|CastToTTTPlayerControllerBP NewPlayer))
  (Utilities|Array|Add (Variables|Default|GetPlayerControllerList) _astttplayer_controller_bp)
  (Default|AuthenticatePlayer _astttplayer_controller_bp false)
  (bind _returnvalue (Class|GameModeBase|GetNumPlayers))
  (if (== _returnvalue 2)
    (Development|PrintString "Game Can Be started Now")
    (Utilities|Time|SetTimerbyEvent (delegate Custom|StartGame) 3.0)))

(event EventOnLogout
  (params (ExitingController :type Controller%20Object%20Reference))
  (bind _playercontrollerlist (Variables|Default|GetPlayerControllerList))
  (bind _astttplayer_controller_bp (Utilities|Casting|CastToTTTPlayerControllerBP ExitingController))
  (if (Utilities|Array|ContainsItem _playercontrollerlist _astttplayer_controller_bp)
    (Utilities|Array|RemoveItem _playercontrollerlist _astttplayer_controller_bp)
    (Development|PrintString "Removed PlayerControoler Object After Log Out")))

(fn ConstructionScript)